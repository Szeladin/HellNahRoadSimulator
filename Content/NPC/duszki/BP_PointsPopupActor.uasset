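; BP_PointsPopupActor is a short-lived floating popup that shows a point value through a WBP_PointsPopup widget.
; On BeginPlay the Zanikanie timeline lifts the actor every update by a fixed step plus an alpha-scaled offset, then destroys it when finished.
; Each update also pushes PunktyValue into the widget, negated when Isevil is false, and calls ChangeValue.
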(event `self.ReceiveBeginPlay`
  (bind _defaultsceneroot (`self.DefaultSceneRoot`))
  (bind _punktyvalue (`self.PunktyValue`))
  (bind (_direction _alpha) (`Timeline|zanikanie` :`NewTime` 1.0)
    (:`Update`
      (`SceneComponent.K2_SetWorldLocation` _defaultsceneroot (`KismetMathLibrary.MakeVector` (.x (`SceneComponent.K2_GetComponentLocation` _defaultsceneroot)) (.y (`SceneComponent.K2_GetComponentLocation` _defaultsceneroot)) (+ (.z (`SceneComponent.K2_GetComponentLocation` _defaultsceneroot)) (* _alpha 5.0) 50.0)) false false)
      (`|ExecutionSequence`
        (:`then_0`
          (bind _aswbp_points_popup (cast `/Game/NPC/duszki/WBP_PointsPopup` (`WidgetComponent.GetUserWidgetObject` (`self.Punkty`))))
          (if (`self.isevil`)
            (set `/Game/NPC/duszki/WBP_PointsPopup.Point` _punktyvalue _aswbp_points_popup)
            (`/Game/NPC/duszki/WBP_PointsPopup.ChangeValue` _aswbp_points_popup)
            (else
              (set `/Game/NPC/duszki/WBP_PointsPopup.Point` (* _punktyvalue -1) _aswbp_points_popup)
              (`/Game/NPC/duszki/WBP_PointsPopup.ChangeValue` _aswbp_points_popup))))))
    (:`Finished`
      (`self.K2_DestroyActor`))))

(event `self.ReceiveTick`
  (params (DeltaSeconds :type "Float (single-precision)")))

(fn `UserConstructionScript`)