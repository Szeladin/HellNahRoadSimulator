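; Manager actor that keeps a capped population of good and evil ghosts around the player and handles their scoring.
; A fast looping timer line-traces downward near random points around the pawn and spawns a random ghost type on hits, registering itself as its Manager.
; A slower timer culls ghosts too far from the player controller.
; DestroyGhost removes a ghost, adding random points for evil ones and subtracting them for others via the vehicle player controller.
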(event `self.ReceiveBeginPlay`
  (set `self.MaxGhost` 400)
  (set `self.SpawnRadiusMax` 50000.0)
  (set `self.SpawnRadiusMin` 500.0)
  (set `self.DespawnDistance` 70000.0)
  (bind _output_get (set `self.SpawnInterval` 0.1))
  (`|ExecutionSequence`
    (:`then_0`
      (`KismetSystemLibrary.K2_SetTimerDelegate` (delegate `Try spawn Ghost`) _output_get true))
    (:`then_1`
      (`KismetSystemLibrary.K2_SetTimerDelegate` (delegate `Check despawn`) 1.0 true))))

(event `Try spawn Ghost`
  (bind _returnvalue (+ (`self.K2_GetActorLocation` (`GameplayStatics.GetPlayerPawn` 0)) (* (`KismetMathLibrary.RandomFloatInRange` (`self.SpawnRadiusMin`) (`self.SpawnRadiusMax`)) (`KismetMathLibrary.RandomUnitVector`))))
  (if (> (`self.MaxGhost`) (`KismetArrayLibrary.Array_Length` (`self.ActiveGhosts`)))
    (bind (_outhit _returnvalue_2) (`KismetSystemLibrary.LineTraceSingle` (+ _returnvalue (0.0 0.0 500.0)) (- _returnvalue (0.0 0.0 20000.0)) "TraceTypeQuery1"))
    (if _returnvalue_2
      (switch `int` (`KismetMathLibrary.RandomIntegerInRange` 1 2)
        (:`Default`
          (bind _asbp_ghost (castclass `/Game/NPC/duszki/BP_Ghost` "/Game/NPC/duszki/BP_Ghost_Good.BP_Ghost_Good_C" :!label _label))
          (bind _returnvalue_3 (`KismetMathLibrary.Conv_VectorToTransform` (+ (`.Location` (`GameplayStatics.BreakHitResult` _outhit)) (0.0 0.0 100.0))))
          (bind _returnvalue_4 (`|SpawnActorFromClass` _asbp_ghost _returnvalue_3 "Undefined" "MultiplyWithRoot" null null))
          (set `/Game/NPC/duszki/BP_Ghost.Manager` self _returnvalue_4)
          (`KismetArrayLibrary.Array_Add` (`self.ActiveGhosts`) _returnvalue_4))
        (:`1`
          (goto _label))
        (:`2`
          (bind _asbp_ghost_2 (castclass `/Game/NPC/duszki/BP_Ghost` "/Game/NPC/duszki/BP_Ghost_Evil.BP_Ghost_Evil_C"))
          (bind _returnvalue_5 (`|SpawnActorFromClass` _asbp_ghost_2 _returnvalue_3 "Undefined" "MultiplyWithRoot" null null))
          (set `/Game/NPC/duszki/BP_Ghost.Manager` self _returnvalue_5)
          (`KismetArrayLibrary.Array_Add` (`self.ActiveGhosts`) _returnvalue_5))))))

(event `Check despawn`
  (for _array_element (`self.ActiveGhosts`)
    (`/Engine/EditorBlueprintResources/StandardMacros.IsValid` _array_element
      (:`Is Valid`
        (if (> (`KismetMathLibrary.Vector_Distance` (`self.K2_GetActorLocation` _array_element) (`self.K2_GetActorLocation` (`GameplayStatics.GetPlayerController` 0))) (`self.DespawnDistance`))
          (`self.K2_DestroyActor` _array_element)
          (`KismetArrayLibrary.Array_RemoveItem` (`self.ActiveGhosts`) _array_element))))))

(event `DestroyGhost`
  (params (Item :type "/Game/NPC/duszki/BP_Ghost Object Reference (by ref)"))
  (bind _returnvalue (`KismetMathLibrary.RandomInteger` 100))
  (`self.SetActorTickEnabled` Item false)
  (`|ExecutionSequence`
    (:`then_0`
      (bind _asbp_vehicle_adv_player_controller (cast `/Game/VehicleTemplate/Blueprints/BP_VehicleAdvPlayerController` (`GameplayStatics.GetPlayerController` 0)))
      (`KismetSystemLibrary.IsObjectOfSoftClass` Item "/Game/NPC/duszki/BP_Ghost_Evil.BP_Ghost_Evil_C"
        (:`True`
          (`/Game/VehicleTemplate/Blueprints/BP_VehicleAdvPlayerController.AddPoints` _asbp_vehicle_adv_player_controller _returnvalue))
        (:`False`
          (`/Game/VehicleTemplate/Blueprints/BP_VehicleAdvPlayerController.AddPoints` _asbp_vehicle_adv_player_controller (* _returnvalue -1)))))
    (:`then_1`
      (`self.K2_DestroyActor` Item)
      (`KismetArrayLibrary.Array_RemoveItem` (`self.ActiveGhosts`) Item))))

(fn `UserConstructionScript`)