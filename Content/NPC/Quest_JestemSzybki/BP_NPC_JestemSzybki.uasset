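; Quest-giver NPC for "Jestem szybki!", a timed checkpoint trial, which pins itself to a fixed world transform on BeginPlay.
; Overlapping its Kolizje component writes a quest struct with hardcoded absolute checkpoint transforms, checkpoint class, time limit and reward into the vehicle player controller's MozliwyQuest.
; It also flags a quest as nearby; actor end overlap clears that flag through the controller reference cast on begin overlap.
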(event `self.ReceiveBeginPlay`
  (`self.K2_SetActorLocationAndRotation` (-79380.0 126140.0 9257.0) (`KismetMathLibrary.MakeRotator` 0.0 0.0 176.0))
  (`self.SetActorScale3D` (1.2 1.2 1.2)))

(event `self.Kolizje.OnComponentBeginOverlap`
  (params (OverlappedComponent :type "PrimitiveComponent Object Reference") (OtherActor :type "Actor Object Reference") (OtherComp :type "PrimitiveComponent Object Reference") (OtherBodyIndex :type Integer) (bFromSweep :type Boolean) (SweepResult :type "HitResult Structure (by ref)"))
  ; ustawianie questa
  (bind _asitem_to_collect (castclass `/Game/Quest/Znajdzki/ItemToCollect` "/Game/Quest/Znajdzki/JestemSzybki/JestemSzybki_PunktKontrolny.JestemSzybki_PunktKontrolny_C"))
  (bind _asbp_vehicle_adv_player_controller (cast `/Game/VehicleTemplate/Blueprints/BP_VehicleAdvPlayerController` (`GameplayStatics.GetPlayerController` 0)))
  (set `/Game/VehicleTemplate/Blueprints/BP_VehicleAdvPlayerController.MozliwyQuest` (make `/Game/Quest/ST_Quest` 2 "Jestem szybki!" "Witaj wędrowcze" "NewEnumerator0" 12 2500 "Należy ukończyć próbę czasową" (`|MakeArray` (`KismetMathLibrary.MakeTransform` (-100710.0 117950.0 9520.0) (struct :`Yaw` 155.0) (5.0 5.0 5.0)) (`KismetMathLibrary.MakeTransform` (-75494.935127 80219.017104 355.189503) (struct :`Yaw` -121.0) (5.0 5.0 5.0)) (`KismetMathLibrary.MakeTransform` (-64934.935127 69879.017104 355.189503) (struct :`Yaw` -18.0) (5.0 5.0 5.0)) (`KismetMathLibrary.MakeTransform` (-83324.935127 58609.017104 355.189503) (struct :`Yaw` 91.0) (5.0 5.0 5.0)) (`KismetMathLibrary.MakeTransform` (-129612.498893 62874.763099 9595.919467) (struct :`Yaw` -34.0) (5.0 5.0 5.0)) (`KismetMathLibrary.MakeTransform` (-129642.498893 36784.763099 9355.919467) (struct :`Yaw` -142.0) (5.0 5.0 5.0)) (`KismetMathLibrary.MakeTransform` (-106932.498893 15984.763099 695.919467) (struct :`Yaw` 89.0) (5.0 5.0 5.0)) (`KismetMathLibrary.MakeTransform` (-110952.498893 63034.763099 8625.919467) (struct :`Yaw` 62.0) (5.0 5.0 5.0)) (`KismetMathLibrary.MakeTransform` (-83330.0 126820.0 9520.0) (struct :`Yaw` 100.0) (5.0 5.0 5.0)) (`KismetMathLibrary.MakeTransform` (-105072.498893 9024.763099 95.919467) (struct :`Yaw` -16.0) (5.0 5.0 5.0)) (`KismetMathLibrary.MakeTransform` (-123712.498893 -15125.236901 475.919467) (struct :`Yaw` -32.0) (5.0 5.0 5.0)) (`KismetMathLibrary.MakeTransform` (-124142.498893 -42255.236901 335.919467) (struct :`Yaw` -20.0) (5.0 5.0 5.0))) _asitem_to_collect 120 self "Punkty kontrolne") _asbp_vehicle_adv_player_controller)
  (set `/Game/VehicleTemplate/Blueprints/BP_VehicleAdvPlayerController.isquestnearby` true _asbp_vehicle_adv_player_controller))

(event `self.ReceiveActorEndOverlap`
  (params (OtherActor :type "Actor Object Reference"))
  ; ustawianie questa
  ;; uniemozliwienie zwiecia questa jak nie jest w poblizu
  (set `/Game/VehicleTemplate/Blueprints/BP_VehicleAdvPlayerController.isquestnearby` false (stale `self.Kolizje.OnComponentBeginOverlap` _asbp_vehicle_adv_player_controller)))

(fn `UserConstructionScript`)