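; Quest-giver NPC for "Zaginione Monety" (Lost Coins), a quest to collect nine coins scattered across the map.
; On BeginPlay it snaps to a hard-coded world position and scale.
; Overlapping Kolizje passes an STQuest, with reward, item class and absolute coin transforms, to BP_VehicleAdvPlayerController as the available quest and sets Isquestnearby.
; Actor end overlap clears that flag; neither overlap event checks the other actor.
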(event `self.ReceiveBeginPlay`
  (`self.K2_SetActorLocationAndRotation` (151809.654929 10118.295476 5751.156095) (`KismetMathLibrary.MakeRotator` 0.0))
  (`self.SetActorScale3D` (5.0 5.0 5.0)))

(event `self.Kolizje.OnComponentBeginOverlap`
  (params (OverlappedComponent :type "PrimitiveComponent Object Reference") (OtherActor :type "Actor Object Reference") (OtherComp :type "PrimitiveComponent Object Reference") (OtherBodyIndex :type Integer) (bFromSweep :type Boolean) (SweepResult :type "HitResult Structure (by ref)"))
  ; ustawianie questa
  (bind _asitem_to_collect (castclass `/Game/Quest/Znajdzki/ItemToCollect` "/Game/Quest/Znajdzki/ZaginioneMonety/ZaginioneMonety_1.ZaginioneMonety_1_C"))
  (bind _asbp_vehicle_adv_player_controller (cast `/Game/VehicleTemplate/Blueprints/BP_VehicleAdvPlayerController` (`GameplayStatics.GetPlayerController` 0)))
  (set `/Game/VehicleTemplate/Blueprints/BP_VehicleAdvPlayerController.MozliwyQuest` (make `/Game/Quest/ST_Quest` 0 "Zaginione Monety" "Witaj wędrowcze" "NewEnumerator0" 9 1000 "Do zebrania 9 monet rozrzuconych na mapie" (`|MakeArray` (`KismetMathLibrary.MakeTransform` (147980.784264 12480.436306 6187.286008) (struct) (26.25 26.25 26.25)) (`KismetMathLibrary.MakeTransform` (161580.784264 13160.436306 6187.286008) (struct) (26.25 26.25 26.25)) (`KismetMathLibrary.MakeTransform` (160240.784264 10620.436306 6187.286008) (struct) (26.25 26.25 26.25)) (`KismetMathLibrary.MakeTransform` (160680.784264 -3719.563694 6187.286008) (struct) (26.25 26.25 26.25)) (`KismetMathLibrary.MakeTransform` (178200.784264 7900.436306 7227.286008) (struct :`Pitch` 8.0 :`Roll` -28.0) (26.25 26.25 26.25)) (`KismetMathLibrary.MakeTransform` (167020.784264 21570.436306 6187.286008) (struct) (26.25 26.25 26.25)) (`KismetMathLibrary.MakeTransform` (154480.784264 21080.436306 6187.286008) (struct) (26.25 26.25 26.25)) (`KismetMathLibrary.MakeTransform` (183460.784264 2260.436306 8207.286008) (struct :`Pitch` 38.0 :`Roll` 8.0) (26.25 26.25 26.25)) (`KismetMathLibrary.MakeTransform` (170380.784264 2260.436306 6187.286008) (struct) (26.25 26.25 26.25))) _asitem_to_collect 0 self "Monety") _asbp_vehicle_adv_player_controller)
  (set `/Game/VehicleTemplate/Blueprints/BP_VehicleAdvPlayerController.isquestnearby` true _asbp_vehicle_adv_player_controller))

(event `self.ReceiveActorEndOverlap`
  (params (OtherActor :type "Actor Object Reference"))
  ; ustawianie questa
  ;; uniemozliwienie zwiecia questa jak nie jest w poblizu
  (set `/Game/VehicleTemplate/Blueprints/BP_VehicleAdvPlayerController.isquestnearby` false (stale `self.Kolizje.OnComponentBeginOverlap` _asbp_vehicle_adv_player_controller)))

(fn `UserConstructionScript`)