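; NPC quest giver for "Nie odpala" ("Won't start"), a towing quest to bring a car to a gas station.
; Overlapping its Kolizje component writes a hardcoded quest struct, with target class, locations and reward, to the vehicle player controller and flags a quest as nearby.
; Ending actor overlap clears that flag, so the quest cannot be taken from afar.
; A custom event moves and rescales the NPC to a fixed spot.
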(event `CustomEvent`
  (`self.K2_SetActorLocationAndRotation` (-25720.0 77630.0 50.0) (`KismetMathLibrary.MakeRotator` 0.0))
  (`self.SetActorScale3D` (2.5 2.5 2.5)))

(event `self.Kolizje.OnComponentBeginOverlap`
  (params (OverlappedComponent :type "PrimitiveComponent Object Reference") (OtherActor :type "Actor Object Reference") (OtherComp :type "PrimitiveComponent Object Reference") (OtherBodyIndex :type Integer) (bFromSweep :type Boolean) (SweepResult :type "HitResult Structure (by ref)"))
  ; ustawianie questa
  (bind _asitem_to_collect (castclass `/Game/Quest/Znajdzki/ItemToCollect` "/Game/Quest/Znajdzki/NieOdpala/NieOdpala_Cel.NieOdpala_Cel_C"))
  (bind _asbp_vehicle_adv_player_controller (cast `/Game/VehicleTemplate/Blueprints/BP_VehicleAdvPlayerController` (`GameplayStatics.GetPlayerController` 0)))
  (set `/Game/VehicleTemplate/Blueprints/BP_VehicleAdvPlayerController.MozliwyQuest` (make `/Game/Quest/ST_Quest` 1 "Nie odpala" "Witaj wędrowcze" "NewEnumerator1" 2 2000 "Zawieź samochód na najbliższą stację benzynową" (`|MakeArray` (`KismetMathLibrary.MakeTransform` (90800.0 -69180.0 6530.0) (struct) (4.0 4.0 4.0)) (`KismetMathLibrary.MakeTransform` (-25110.0 77660.0 180.0) (struct) (2.0 2.0 2.0)) (struct)) _asitem_to_collect 0 self "Zawieź pojazd na stację benzynową obok UBB" true) _asbp_vehicle_adv_player_controller)
  (set `/Game/VehicleTemplate/Blueprints/BP_VehicleAdvPlayerController.isquestnearby` true _asbp_vehicle_adv_player_controller))

(event `self.ReceiveActorEndOverlap`
  (params (OtherActor :type "Actor Object Reference"))
  ; ustawianie questa
  ;; uniemozliwienie zwiecia questa jak nie jest w poblizu
  (set `/Game/VehicleTemplate/Blueprints/BP_VehicleAdvPlayerController.isquestnearby` false (stale `self.Kolizje.OnComponentBeginOverlap` _asbp_vehicle_adv_player_controller)))

(fn `UserConstructionScript`)