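; Quest manager Blueprint that holds the list of all quests and tracks which one is active.
; BeginPlay clears the active state, and AddQuest appends entries to the AllQuests array.
; SetActiveQuestByID stores the ID found by a linear lookup and flags a quest as active, with no check that the lookup succeeded.
; GetActiveQuest searches the array for that ID and returns the quest data with a validity flag.
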(event `self.ReceiveBeginPlay`
  (set `self.HasActiveQuest` false)
  (set `self.ActiveQuestID` -1))

(fn `AddQuest`
  (params (NewItem :type "/Game/Quest/ST_QuestData Structure (by ref)"))
  (`KismetArrayLibrary.Array_Add` (`self.AllQuests`) NewItem))

(fn `GetActiveQuest`
  (returns (QuestData :type "/Game/Quest/ST_QuestData Structure") (IsValid :type Boolean))
  (if (`self.HasActiveQuest`)
    (for _array_element (`self.AllQuests`)
      (if (== (`self.ActiveQuestID`) (`.QuestID_2_EF14FD7445D0A626763502BC6D618266` (break `/Game/Quest/ST_QuestData` _array_element)))
        (return _array_element true)))
    (return (struct) false)))

(fn `GetQuestByID`
  (params (QuestID :type Integer))
  (returns (QuestByID :type "/Game/Quest/ST_QuestData Structure"))
  (locals (LoopItem :type "/Game/Quest/ST_QuestData Structure"))
  (for _array_element (`self.AllQuests`)
    (if (== (`.QuestID_2_EF14FD7445D0A626763502BC6D618266` (break `/Game/Quest/ST_QuestData` _array_element)) QuestID)
      (return _array_element))))

(fn `setActiveQuestByID`
  (params (QuestID :type Integer))
  (bind _questbyid (`self.GetQuestByID` QuestID))
  (set `self.ActiveQuestID` (`.QuestID_2_EF14FD7445D0A626763502BC6D618266` (break `/Game/Quest/ST_QuestData` _questbyid)))
  (set `self.HasActiveQuest` true))

(fn `UserConstructionScript`)