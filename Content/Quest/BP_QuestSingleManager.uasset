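; BP_QuestSingleManager is an actor that holds and tracks the state of a single quest.
; LoadQuest stores the quest data and resets progress, timer and completion; StartQuest activates it, enabling the countdown only for Collect quests.
; Tick decrements the remaining time and flags failure at zero, without calling FailQuest or deactivating the quest.
; CompliteQuest and FailQuest deactivate the quest, with completion returning its reward points.
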(event `self.ReceiveTick`
  (params (DeltaSeconds :type "Float (single-precision)"))
  (if (and (`self.IsQuestActive`) (`self.StatTime`))
    (bind _output_get (set `self.RemainingTime` (- (`self.RemainingTime`) DeltaSeconds)))
    (if (<= _output_get 0.0)
      (set `self.IsFailed` true))))

(fn `CompliteQuest`
  (returns (Points :type Integer))
  (set `self.IsQuestActive` false)
  (set `self.IsCompleted` true)
  (return (`.RewardPoints_20_DA27DF6E41BC8E4AE979EDA6E36EAE3F` (break `/Game/Quest/ST_QuestData` (`self.CurrnetQuestData`)))))

(fn `FailQuest`
  (set `self.IsFailed` true)
  (set `self.IsQuestActive` false))

(fn `LoadQuest`
  (params (CurrnetQuestData :type "/Game/Quest/ST_QuestData Structure"))
  (bind _output_get (set `self.CurrnetQuestData` CurrnetQuestData))
  (set `self.CurrentProgress` 0)
  (set `self.RemainingTime` (`.TimeLimit_19_2D3BAAEE4CF19847AA78CE83C823A4F1` (break `/Game/Quest/ST_QuestData` _output_get)))
  (set `self.IsCompleted` false)
  (set `self.IsQuestActive` false)
  (set `self.StatTime` false))

(fn `StartQuest`
  (set `self.IsQuestActive` true)
  (switch `/Game/Quest/QuestType` (`.QuestType_12_9CDD09664EB12CE225B7C39B3E6FADDB` (break `/Game/Quest/ST_QuestData` (`self.CurrnetQuestData`)))
    (:`NewEnumerator0`
      (set `self.StatTime` true))))

(fn `UserConstructionScript`)